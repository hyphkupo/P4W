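; BP_DemoVFX is a demo actor that showcases the Niagara effects of the ClawAttackVFX content one after another.
; On BeginPlay it takes over the player's view, then loops every two seconds, spawning the next array entry attached to its root.
; The index increments with no wrap or bounds check.
; Tick slowly yaws the spring arm by a fixed per-frame step, independent of delta time.
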(event EventTick
  (params (DeltaSeconds :type Float%20%28single-precision%29))
  (Transformation|AddRelativeRotation (Variables|Default|GetSpringArm) "0,0.250000, 0" false false))

(event EventBeginPlay
  (Game|Player|SetViewTargetwithBlend (Game|GetPlayerController 0) self 0.0 "VTBlend_Linear" 0.0 false)
  (Utilities|FlowControl|Delay 2.0 :!label _label)
  (Niagara|SpawnSystemAttached (Utilities|Array|Get(acopy) (Variables|Default|GetNiagara) (Variables|Default|Getindex)) (Variables|Default|GetDefaultSceneRoot) "None" "0, 0, 0" "0, 0, 0" "KeepRelativeOffset" false)
  (Math|Integer|IncrementInt (Variables|Default|Getindex)
    (:%20%20
      (goto _label))))

(fn ConstructionScript)